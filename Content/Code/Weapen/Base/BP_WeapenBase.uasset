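; Base weapon actor that handles automatic hitscan firing, ammo and reloading for the player.
; A looping timer drives FireInternal, which plays state-based weapon and arm montages, muzzle effects, casing ejection and recoil, then camera-traces to spawn surface-specific impacts and decals without applying damage.
; A weapon state gates firing and reloading; Reload only plays montages and sound, while ReloadAmmo, uncalled here, moves reserve ammo into the magazine.
; Tick prints ammo counts for debugging.
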(event Custom|Fire%20Internal
  (bind _player (Variables|Default|GetPlayer))
  (bind _weapen (Variables|Default|GetWeapen))
  (bind _returnvalue (Transformation|GetSocketTransform _weapen "Casing" "RTS_World"))
  (bind _camera (Variables|/Game/Code/Player/BP_FPSplayer.BP_FPSplayer_C|GetCamera _player))
  (bind _returnvalue_2 (Transformation|GetWorldLocation _camera))
  (if (<= (Variables|Default|GetCurrentAmmo) 0)
    (CallFunction|StopFire)
    (else
      (Animation|Montage|PlayMontage (Variables|Default|GetWeapen) (Utilities|Select :Index (Variables|/Game/Code/Player/BP_FPSplayer.BP_FPSplayer_C|GetE_PlayerState (Variables|Default|GetPlayer)) :NewEnumerator0 (Variables|Default|GetWeaponIdle) :NewEnumerator1 (Variables|Default|GetWeaponWalk) :NewEnumerator2 0 :NewEnumerator3 (Variables|Default|GetWeaponAim))
        (:then
          (Animation|Montage|PlayMontage (Variables|/Game/Code/Player/BP_FPSplayer.BP_FPSplayer_C|GetArm (Variables|Default|GetPlayer)) (Utilities|Select :Index (Variables|/Game/Code/Player/BP_FPSplayer.BP_FPSplayer_C|GetE_PlayerState (Variables|Default|GetPlayer)) :NewEnumerator0 (Variables|Default|GetPlayerIdle) :NewEnumerator1 (Variables|Default|GetPlayerWalk) :NewEnumerator2 0 :NewEnumerator3 (Variables|Default|GetPlayerAim))
            (:then
              (Audio|PlaySound2D "/Game/Code/Weapen/MetaSound/MS_VIRTUS.MS_VIRTUS" 1.0 1.0 0.0 "/Game/Code/Weapen/MetaSound/SC_WeaponFire.SC_WeaponFire" 0)
              (Niagara|SpawnSystemAttached "/Game/ShotSystem/Shot_VFX/VIRTUS_MuzzleFlash.VIRTUS_MuzzleFlash" (Variables|Default|GetBarrel) "Muzzle" "0, 0, 0" "0, 0, 0" "KeepRelativeOffset" true)
              (Math|Integer|DecrementInt (Variables|Default|GetCurrentAmmo)
                (:%20%20
                  (Game|SpawnActorfromClass "/Game/Code/Weapen/BP_Casing.BP_Casing_C" (Math|Transform|MakeTransform (.location _returnvalue) (.rotation _returnvalue) "1.000000,1.000000,1.000000") "Undefined" "MultiplyWithRoot" 0 0)
                  (Pawn|Input|AddControllerPitchInput (Variables|Default|GetPlayer) -0.4)
                  (Pawn|Input|AddControllerYawInput (Variables|Default|GetPlayer) (Math|Random|RandomFloatinRange -0.1 0.1))
                  (bind _outhit (Collision|LineTraceByChannel _returnvalue_2 (+ _returnvalue_2 (* (Math|Vector|GetForwardVector _camera) 10000)) "TraceTypeQuery1" false 0 "None"))
                  (if (.bBlockingHit (Collision|BreakHitResult _outhit))
                    (Variables|Default|SetLineLocation (.Location (Collision|BreakHitResult _outhit)))
                    (Variables|Default|SetLineRotation (Math|Rotator|MakeRotfromX (.Normal (Collision|BreakHitResult _outhit))))
                    (switch Utilities|FlowControl|Switch|SwitchonEPhysicalSurface (Variables|/Script/PhysicsCore.PhysicalMaterial|GetSurfaceType (.PhysMat (Collision|BreakHitResult _outhit)))
                      (:SurfaceType_Default
                        (Niagara|SpawnSystematLocation "/Game/ShotSystem/Shot_VFX/FX_SquibConcrete.FX_SquibConcrete" (Variables|Default|GetLineLocation) (Variables|Default|GetLineRotation) :!label _label)
                        (Audio|PlaySoundatLocation "/Game/XL_FPSPack/Common/Sound/Bullet_Impact_Sounds/Concrete/Hit_Concrete.Hit_Concrete" (Variables|Default|GetLineLocation) "0, 0, 0" 0.6 1.0 0.0 0 0 0 0)
                        (bind _returnvalue_3 (Game|SpawnActorfromClass "/Game/Decals/BP_BulletDecal.BP_BulletDecal_C" (Math|Transform|MakeTransform (Variables|Default|GetLineLocation) (Variables|Default|GetLineRotation) "0.400000,0.400000,0.400000") "Undefined" "MultiplyWithRoot" 0 0))
                        (Rendering|Components|Decal|SetDecalMaterial (Variables|/Game/Decals/BP_BulletDecal.BP_BulletDecal_C|GetBulletDecal _returnvalue_3) "/Game/Decals/Materials/MI_VFX_BulletDecal_Concrete.MI_VFX_BulletDecal_Concrete"))
                      (:SurfaceType1
                        (Niagara|SpawnSystematLocation "/Game/XL_FPSPack/Niagara_VFX/Niagara/Blood/Blood_Splat.Blood_Splat" (Variables|Default|GetLineLocation) (Variables|Default|GetLineRotation))
                        (Audio|PlaySoundatLocation "/Game/XL_FPSPack/Common/Sound/Bullet_Impact_Sounds/Concrete/Hit_Concrete.Hit_Concrete" (Variables|Default|GetLineLocation) "0, 0, 0" 0.6 1.0 0.0 0 0 0 0)
                        (Game|SpawnActorfromClass "/Game/Decals/BP_BulletDecal.BP_BulletDecal_C" (Math|Transform|MakeTransform (Variables|Default|GetLineLocation) (Variables|Default|GetLineRotation) "0.400000,0.400000,0.400000") "Undefined" "MultiplyWithRoot" 0 0))
                      (:SurfaceType2
                        (Niagara|SpawnSystematLocation "/Game/XL_FPSPack/Niagara_VFX/Niagara/Impact/Impact_Wood.Impact_Wood" (Variables|Default|GetLineLocation) (Variables|Default|GetLineRotation))
                        (Audio|PlaySoundatLocation "/Game/ShotSystem/Shot_SFX/SFX_Vefects_Shots_Squib_Wood_Cue.SFX_Vefects_Shots_Squib_Wood_Cue" (Variables|Default|GetLineLocation) "0, 0, 0" 1.6 1.0 0.0 0 0 0 0)
                        (bind _returnvalue_4 (Game|SpawnActorfromClass "/Game/Decals/BP_BulletDecal.BP_BulletDecal_C" (Math|Transform|MakeTransform (Variables|Default|GetLineLocation) (Variables|Default|GetLineRotation) "0.400000,0.400000,0.400000") "Undefined" "MultiplyWithRoot" 0 0))
                        (Rendering|Components|Decal|SetDecalMaterial (Variables|/Game/Decals/BP_BulletDecal.BP_BulletDecal_C|GetBulletDecal _returnvalue_4) "/Game/Decals/Materials/MI_VFX_BulletDecal_Wood.MI_VFX_BulletDecal_Wood"))
                      (:SurfaceType3
                        (Niagara|SpawnSystematLocation "/Game/ShotSystem/Shot_VFX/FX_SquibDirt.FX_SquibDirt" (Variables|Default|GetLineLocation) (Variables|Default|GetLineRotation))
                        (Audio|PlaySoundatLocation "/Game/ShotSystem/Shot_SFX/SFX_Vefects_Shots_Squib_Dirt_Cue.SFX_Vefects_Shots_Squib_Dirt_Cue" (Variables|Default|GetLineLocation) "0, 0, 0" 1.0 1.0 0.0 0 0 0 0)
                        (Game|SpawnActorfromClass "/Game/Decals/BP_BulletDecal.BP_BulletDecal_C" (Math|Transform|MakeTransform (Variables|Default|GetLineLocation) (Variables|Default|GetLineRotation) "0.400000,0.400000,0.400000") "Undefined" "MultiplyWithRoot" 0 0))
                      (:SurfaceType4
                        (Niagara|SpawnSystematLocation "/Game/ShotSystem/Shot_VFX/FX_SquibMetal.FX_SquibMetal" (Variables|Default|GetLineLocation) (Variables|Default|GetLineRotation))
                        (Audio|PlaySoundatLocation "/Game/ShotSystem/Shot_SFX/SFX_Vefects_Shots_Squib_Metal_Cue.SFX_Vefects_Shots_Squib_Metal_Cue" (Variables|Default|GetLineLocation) "0, 0, 0" 1.6 1.0 0.0 0 0 0 0)
                        (bind _returnvalue_5 (Game|SpawnActorfromClass "/Game/Decals/BP_BulletDecal.BP_BulletDecal_C" (Math|Transform|MakeTransform (Variables|Default|GetLineLocation) (Variables|Default|GetLineRotation) "0.400000,0.400000,0.400000") "Undefined" "MultiplyWithRoot" 0 0))
                        (Rendering|Components|Decal|SetDecalMaterial (Variables|/Game/Decals/BP_BulletDecal.BP_BulletDecal_C|GetBulletDecal _returnvalue_5) "/Game/Decals/Materials/MI_VFX_BulletDecal_Metal.MI_VFX_BulletDecal_Metal"))
                      (:SurfaceType5
                        (goto _label)))))))))))))

(event Custom|stop%20fire
  (switch Utilities|FlowControl|Switch|SwitchonE_WeaponState (Variables|Default|GetWeaponState)
    (:NewEnumerator0
      _)
    (:NewEnumerator1
      _))
  (Utilities|Time|ClearandInvalidateTimerbyHandle (Variables|Default|GetFiretimeHandle))
  (Variables|Default|SetWeaponState "NewEnumerator0"))

(event Custom|Reload
  (params (目标 :type BP%20FP%20Splayer%20Object%20Reference))
  (switch Utilities|FlowControl|Switch|SwitchonE_WeaponState (Variables|Default|GetWeaponState)
    (:NewEnumerator0
      (if (and (< (Variables|Default|GetCurrentAmmo) (Variables|Default|GetMagSize)) (> (Variables|Default|GetTotalAmmo) 0))
        (Variables|Default|SetWeaponState "NewEnumerator2")
        (Animation|Montage|PlayMontage (Variables|Default|GetWeapen) "/Game/XL_FPSPack/Weapons/MCX-VIRTUS/Animation/Weapon/Weapon_MCX-VIRTUS_Reload_Empty_Montage.Weapon_MCX-VIRTUS_Reload_Empty_Montage"
          (:then
            (Animation|Montage|PlayMontage (Variables|/Game/Code/Player/BP_FPSplayer.BP_FPSplayer_C|GetArm 目标) "/Game/XL_FPSPack/Weapons/MCX-VIRTUS/Animation/Player/Player_MCX-VIRTUS_Reload_Empty_Montage.Player_MCX-VIRTUS_Reload_Empty_Montage"
              (:then
                (Audio|PlaySound2D "/Game/XL_FPSPack/Weapons/MCX-VIRTUS/Sound/Foley/SW_MCX-VIRTUS_Reload_Empty_Foley.SW_MCX-VIRTUS_Reload_Empty_Foley" 1.0 1.0 0.0 0 0))
              (:OnCompleted
                (Variables|Default|SetWeaponState "NewEnumerator0" :!label _label))
              (:OnBlendOut
                (goto _label)))))))))

(event EventBeginPlay)

(event Collision|EventActorBeginOverlap
  (params (OtherActor :type Actor%20Object%20Reference)))

(event EventTick
  (params (DeltaSeconds :type Float%20%28single-precision%29))
  (Development|PrintString (Utilities|String|Append (Utilities|String|Append "当前弹夹" (Utilities|String|ToString(Integer) (Variables|Default|GetCurrentAmmo))) (Utilities|String|Append "所有备弹" (Utilities|String|ToString(Integer) (Variables|Default|GetTotalAmmo)))) true true "(R=0.000000,G=0.660000,B=1.000000,A=1.000000)" 0.0))

(event EventStartWeapenFire
  (params (Player :type BP%20FP%20Splayer%20Object%20Reference))
  (Variables|Default|SetPlayer Player)
  (switch Utilities|FlowControl|Switch|SwitchonE_WeaponState (Variables|Default|GetWeaponState)
    (:NewEnumerator0
      (if (> (Variables|Default|GetCurrentAmmo) 0)
        (CallFunction|FireInternal)
        (bind _returnvalue (Utilities|Time|SetTimerbyEvent (delegate Custom|Fire%20Internal) (Variables|Default|GetFireRate) true))
        (Variables|Default|SetFiretimeHandle _returnvalue)
        (Variables|/Game/Code/Player/BP_FPSplayer.BP_FPSplayer_C|SetIsFiring (Variables|Default|GetPlayer) true)
        (Variables|Default|SetWeaponState "NewEnumerator1")
        (else
          (Audio|PlaySound2D "/Game/XL_FPSPack/Weapons/Common/Sounds/Trigger/Dead_trigger/Hand-Guns/Dead_Trigger_Hand-Guns.Dead_Trigger_Hand-Guns" 1.0 1.0 0.0 0 0))))))

(fn ConstructionScript)

(fn GetAimSocketLocation
  (bind _output_get (Variables|Default|SetAimSocketLocation (Transformation|GetSocketLocation (Variables|Default|GetWeapen) "AimSocket")))
  (return _output_get))

(fn ReloadAmmo
  (if (>= (Variables|Default|GetTotalAmmo) (- (Variables|Default|GetMagSize) (Variables|Default|GetCurrentAmmo)))
    (Variables|Default|SetTotalAmmo (- (Variables|Default|GetTotalAmmo) (- (Variables|Default|GetMagSize) (Variables|Default|GetCurrentAmmo))))
    (Variables|Default|SetCurrentAmmo (Variables|Default|GetMagSize))
    (else
      (Variables|Default|SetCurrentAmmo (+ (Variables|Default|GetCurrentAmmo) (Variables|Default|GetTotalAmmo)))
      (Variables|Default|SetTotalAmmo 0))))