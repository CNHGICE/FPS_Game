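; First-person player character that handles Enhanced Input movement, look, run and aim, and carries a BP_VIRTUS weapon.
; On BeginPlay it adds the input mapping context and spawns the weapon attached to Arm.
; Each Tick aligns Arm to control rotation, derives an Idle/Walk/Run/Aim state from input and velocity, then sets walk speed from it.
; Aim overrides everything, and Run requires forward input, which is zeroed manually on move release.
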(event Input|EnhancedActionEvents|EnhancedInputActionIA_Move
  (params (ActionValue :type Vector%202D%20Structure) (ElapsedSeconds :type Float%20%28double-precision%29) (TriggeredSeconds :type Float%20%28double-precision%29) (InputAction :type Input%20Action%20Object%20Reference :default "/Game/Code/Player/System/Input/IA_Move.IA_Move"))
  (bind (_x _y) (Math|Vector2D|BreakVector2D ActionValue))
  (:Triggered
    (bind _output_get (Variables|Default|SetMove%20X _x))
    (Pawn|Input|AddMovementInput (Math|Vector|GetForwardVector (Math|Rotator|MakeRotator 0.0 0.0 (.yaw (Pawn|GetControlRotation :!class /Script/Engine.Pawn)))) _output_get false)
    (bind _output_get_2 (Variables|Default|SetMove%20Y _y))
    (Pawn|Input|AddMovementInput (Math|Vector|GetRightVector (Math|Rotator|MakeRotator 0.0 0.0 (.yaw (Pawn|GetControlRotation :!class /Script/Engine.Pawn)))) _output_get_2 false))
  (:Completed
    ;[0.15 0.15 0.15 0.5] 手动归零，在完成后方便做奔跑，不然速度没变
    (Variables|Default|SetMove%20X 0.0)
    (Variables|Default|SetMove%20Y 0.0)))

(event Input|EnhancedActionEvents|EnhancedInputActionIA_Look
  (params (ActionValue :type Vector%202D%20Structure) (ElapsedSeconds :type Float%20%28double-precision%29) (TriggeredSeconds :type Float%20%28double-precision%29) (InputAction :type Input%20Action%20Object%20Reference :default "/Game/Code/Player/System/Input/IA_Look.IA_Look"))
  (bind (_x _y) (Math|Vector2D|BreakVector2D ActionValue))
  (Pawn|Input|AddControllerYawInput _x)
  (Pawn|Input|AddControllerPitchInput _y))

(event Input|EnhancedActionEvents|EnhancedInputActionIA_Run
  (params (ActionValue :type Boolean) (ElapsedSeconds :type Float%20%28double-precision%29) (TriggeredSeconds :type Float%20%28double-precision%29) (InputAction :type Input%20Action%20Object%20Reference :default "/Game/Code/Player/System/Input/IA_Run.IA_Run"))
  (:Triggered
    (Variables|Default|SetWant%20to%20Run true))
  (:Completed
    (Variables|Default|SetWant%20to%20Run false)))

(event Input|EnhancedActionEvents|EnhancedInputActionIA_Aim
  (params (ActionValue :type Boolean) (ElapsedSeconds :type Float%20%28double-precision%29) (TriggeredSeconds :type Float%20%28double-precision%29) (InputAction :type Input%20Action%20Object%20Reference :default "/Game/Code/Player/System/Input/IA_Aim.IA_Aim"))
  (:Triggered
    (Variables|Default|SetWant%20to%20Aim true))
  (:Completed
    (Variables|Default|SetWant%20to%20Aim false)))

(event EventBeginPlay
  (bind _as玩家控制器 (Utilities|Casting|CastToPlayerController (Pawn|GetController)))
  (Input|AddMappingContext (PlayerController|LocalPlayerSubsystems|GetEnhancedInputLocalPlayerSubsystem _as玩家控制器) "/Game/Code/Player/System/Input/IMC_FPSInput.IMC_FPSInput" 0 "(bIgnoreAllPressedKeysUntilRelease=True,bForceImmediately=False,bNotifyUserSettings=False)")
  (CallFunction|SpawnWeapen))

(event EventTick
  (params (DeltaSeconds :type Float%20%28single-precision%29))
  (bind _returnvalue (Pawn|GetControlRotation :!class /Script/Engine.Pawn))
  (Transformation|SetWorldRotation (Variables|Default|GetArm) (Math|Rotator|MakeRotator 0.0 (.pitch _returnvalue) (.yaw _returnvalue)) false false)
  (CallFunction|UpdatePlayerState)
  (CallFunction|UpdateMoveSpeed))

(fn ConstructionScript)

(fn UpdatePlayerState
  (if (Variables|Default|GetWant%20to%20Aim)
    (Variables|Default|SetE_PlayerState "NewEnumerator3")
    (elif (> (Variables|Default|GetMove%20X) 0.0)
      (if (Variables|Default|GetWant%20to%20Run)
        (Variables|Default|SetE_PlayerState "NewEnumerator2")
        (else
          (Variables|Default|SetE_PlayerState "NewEnumerator1")))
      (elif (> (Math|Vector|VectorLength (Variables|/Script/Engine.MovementComponent|GetVelocity (Variables|Character|GetCharacterMovement))) 0.0)
        (Variables|Default|SetE_PlayerState "NewEnumerator1")
        (else
          (Variables|Default|SetE_PlayerState "NewEnumerator0"))))))

(fn UpdateMoveSpeed
  (Variables|/Script/Engine.CharacterMovementComponent|SetMaxWalkSpeed (Variables|Character|GetCharacterMovement) (Utilities|Select :Index (Variables|Default|GetE_PlayerState) :NewEnumerator0 4e+02 :NewEnumerator1 4e+02 :NewEnumerator2 6e+02 :NewEnumerator3 265.0)))

(fn SpawnWeapen
  (bind _returnvalue (Game|SpawnActorfromClass "/Game/Code/Weapen/BP_VIRTUS.BP_VIRTUS_C" (Math|Transform|MakeTransform "0, 0, 0" "0, 0, 0" "1.000000,1.000000,1.000000") "Undefined" "MultiplyWithRoot" self 0))
  (bind _output_get (Variables|Default|SetWeapen _returnvalue))
  (Transformation|AttachComponentToComponent _output_get (Variables|Default|GetArm) "None" "KeepRelative" "KeepRelative" "KeepRelative" true))